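; BP_TetrisBlockSpawner is an actor that drops random Tetris blocks into the TetrisFighter level at regular intervals.
; It spawns one block on BeginPlay, and a Tick-driven countdown clears the tracked block reference and spawns again, resetting to ten seconds.
; Each block class is picked randomly from TetrisBlocksToSpawn and placed at the spawner's X, Z and rotation with a random world Y within a fixed range.
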(event `self.ReceiveBeginPlay`
  (`self.AttemptToSpawn`))

(event `self.ReceiveTick`
  (params (DeltaSeconds :type "Float (single-precision)"))
  (bind _output_get (set `self.TetrisBlockSpawnDelay` (- (`self.TetrisBlockSpawnDelay`) DeltaSeconds)))
  (if (<= _output_get 0.0)
    (set `self.CurrentTetrisBlock` null)
    (`self.AttemptToSpawn`)
    (set `self.TetrisBlockSpawnDelay` 10.0)))

(fn `AttemptToSpawn`
  (`/Engine/EditorBlueprintResources/StandardMacros.IsValid` (`self.CurrentTetrisBlock`)
    (:`Is Not Valid`
      (`self.SpawnTetrisBlock`))))

(fn `SpawnTetrisBlock`
  (bind _tetrisblockstospawn (`self.TetrisBlocksToSpawn`))
  (bind _returnvalue (`|SpawnActorFromClass` (`KismetArrayLibrary.Array_Get` _tetrisblockstospawn (`KismetMathLibrary.RandomIntegerInRange` 0 (- (`KismetArrayLibrary.Array_Length` _tetrisblockstospawn) 1))) (`KismetMathLibrary.MakeTransform` (`KismetMathLibrary.MakeVector` (.x (`self.K2_GetActorLocation`)) (`KismetMathLibrary.RandomFloatInRange` -900.0 1100.0) (.z (`self.K2_GetActorLocation`))) (`self.K2_GetActorRotation`)) "AdjustIfPossibleButAlwaysSpawn" "OverrideRootScale"))
  (set `self.CurrentTetrisBlock` _returnvalue))

(fn `UserConstructionScript`)