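; Game mode for TetrisFighter that sets up local players and spawns their side-scroller characters.
; BeginPlay caches all PlayerStart actors and creates local players until the player count exceeds one.
; SpawnCharacter replaces a controller's existing pawn with a SideScrollerCharacter at an indexed start point, possesses it and switches the view to the shared GameCamera.
; The spawn index is then set to 1, so later spawns use the second start point.
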(event `self.ReceiveBeginPlay`
  (bind _numberofplayers (`self.NumberOfPlayers`))
  (bind _outactors (`GameplayStatics.GetAllActorsOfClass` "/Script/Engine.PlayerStart"))
  (set `self.SpawnPoints` _outactors)
  (while (<= _numberofplayers 1)
    (set `self.NumberOfPlayers` (+ _numberofplayers 1))
    (`GameplayStatics.CreatePlayer` -1)))

(event `SpawnCharacter`
  (params (PlayerController :type "PlayerController Object Reference"))
  (bind _returnvalue (`Controller.K2_GetPawn` PlayerController))
  (`/Engine/EditorBlueprintResources/StandardMacros.IsValid` _returnvalue
    (:`Is Valid`
      (`self.K2_DestroyActor` _returnvalue)
      (bind _returnvalue_2 (`|SpawnActorFromClass` "/Game/SideScrollerBP/Blueprints/SideScrollerCharacter.SideScrollerCharacter_C" (`self.GetTransform` (`KismetArrayLibrary.Array_Get` (`self.SpawnPoints`) (`self.NewVar_0`))) "Undefined" "OverrideRootScale"))
      (`Controller.Possess` PlayerController _returnvalue_2)
      (`PlayerController.SetViewTargetWithBlend` PlayerController (`self.GameCamera`) 0.0 "VTBlend_Linear" 0.0 false)
      (set `self.NewVar_0` 1))))

(fn `UserConstructionScript`)